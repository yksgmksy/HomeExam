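; EnemyBP is an enemy that drains health from HeroBP on overlap.
; Overlap start calls DecreaseHero at once and on a looping timer, sending a fixed damage amount through DecreaseHPMessage.
; Overlap end tries to clear "DecreaseHeroHP", which mismatches the timer's "DecreaseHero" function, so the damage loop keeps running.
; BeginPlay initializes the enemy's own Hp and caches the ShooterMode game mode, neither used elsewhere here.
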(event `self.ReceiveBeginPlay`
  (set `self.hp` 100.0)
  (bind _asshooter_mode (cast `/Game/ShooterMode` (`GameplayStatics.GetGameMode`)))
  (set `self.GameMode` _asshooter_mode))

(event `self.ReceiveActorBeginOverlap`
  (params (OtherActor :type "Actor Object Reference"))
  (bind _ashero_bp (cast `/Game/Hero/HeroBP` OtherActor))
  (`self.DecreaseHero`)
  (`KismetSystemLibrary.K2_SetTimer` null "DecreaseHero" 0.2 true))

(event `DecreaseHero`
  (message `/Game/DemageIf.DecreaseHP` (stale `self.ReceiveActorBeginOverlap` _ashero_bp) 20.0))

(event `self.ReceiveActorEndOverlap`
  (params (OtherActor :type "Actor Object Reference"))
  (cast `/Game/Hero/HeroBP` OtherActor)
  (`KismetSystemLibrary.K2_ClearTimer` null "DecreaseHeroHP"))

(fn `UserConstructionScript`)