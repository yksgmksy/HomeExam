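; HeroBP is the player hero of a shooter, with world-axis movement, yaw turning and a gun.
; BeginPlay caches ShooterMode, then spawns GunBP onto the mesh's GunSocket, and BulletTrigger starts and stops its fire.
; DecreaseHP sets Hp to Amount minus Hp (operands reversed from the name's intent) and refreshes the game mode's UI.
; At zero or below, it disables input, destroys gun and hero, and restarts the level by console command.
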(event `self.ReceiveBeginPlay`
  (set `self.hp` 100.0)
  (bind _asshooter_mode (cast `/Game/ShooterMode` (`GameplayStatics.GetGameMode`)))
  (set `self.GameMode` _asshooter_mode)
  (bind _returnvalue (`|SpawnActorFromClass` "/Game/Gun/GunBP.GunBP_C" (`SceneComponent.K2_GetComponentToWorld` (`self.Mesh`)) "Undefined" "OverrideRootScale"))
  (bind _output_get (set `self.Gun` _returnvalue))
  (`self.K2_AttachToComponent` _output_get (`self.Mesh`) "GunSocket" "SnapToTarget" "SnapToTarget" "KeepWorld" true))

(event `InputAxis|MoveForward`
  (params (AxisValue :type "Float (single-precision)"))
  (`self.AddMovementInput` (1.0 0.0 0.0) AxisValue))

(event `InputAction|BulletTrigger`
  (params (Key :type "Key Structure" :default "AnyKey"))
  (bind _gun (`self.Gun`))
  (:`Pressed`
    (`/Game/Gun/GunBP.StartFire` _gun))
  (:`Released`
    (`/Game/Gun/GunBP.StopFire` _gun)))

(event `InputAxis|MoveRight`
  (params (AxisValue :type "Float (single-precision)"))
  (`self.AddMovementInput` (0.0 1.0 0.0) AxisValue))

(event `InputAxis|TurnForward`
  (params (AxisValue :type "Float (single-precision)")))

(event `InputAxis|Turn`
  (params (AxisValue :type "Float (single-precision)"))
  (`self.K2_AddActorLocalRotation` (`KismetMathLibrary.MakeRotator` 0.0 0.0 (* AxisValue 3.0))))

(event `/Game/DemageIf.DecreaseHP`
  (params (amount :type "Float (single-precision)"))
  (bind _output_get (set `self.hp` (- amount (`self.hp`))))
  (`/Game/UI/HUD.UpdateHeroHP` (`/Game/ShooterMode.GameUI` (`self.GameMode`)))
  (if (<= _output_get 0.0)
    (`self.DisableInput` null)
    (`self.K2_DestroyActor` (`self.Gun`))
    (`self.K2_DestroyActor` self)
    (`KismetSystemLibrary.ExecuteConsoleCommand` "restartlevel")))

(fn `UserConstructionScript`)